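; Player actor for a joy-meter game: joy drains each tick at a rate set by game-mode "info" state, drives post-process saturation and triggers a loss below zero.
; Space adds joy scaled by a press counter on a reset timer; clicking actors can decrement it.
; Maxed joy triggers a door knock, voice-volume change and timeline turn from TV to door and back.
; Escape/P toggles pause; balloon spawning is disconnected legacy.
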(event Custom|LookingAtTheDoor
  (if (not (Variables|LookatDoor|GetbIsLookingDoor))
    (Variables|LookatDoor|SetbIsLookingDoor true)
    (Audio|SetSoundMixClassOverride "/Game/MELE/Blueprints/Audio/SCM_Meld.SCM_Meld" "/Game/MELE/Blueprints/Audio/SC_Voice_Meld.SC_Voice_Meld" 0.1 1.0 0.5 true)
    (Utilities|Time|ClearandInvalidateTimerbyHandle (Variables|LookatDoor|GetLookAtDoorHandle))
    (Audio|SpawnSoundatLocation "/Game/MELE/Audios/S_KnockKnock.S_KnockKnock" (Variables|LookatDoor|GetDoorLocation) "0, 0, 0" 1.0 1.0 0.0 0 0)
    (Utilities|FlowControl|Delay 0.5)
    (bind (_direction _alpha) (Timeline|TimeLToDoor PlayFromStart)
      (:Update
        (Transformation|SetActorRotation (Math|Rotator|Lerp(Rotator) "0, 0, 0" (Variables|LookAtDoor|GetRotToDoor) _alpha true)))
      (:Finished
        (if (Utilities|Enum|Equal(Enum) _direction "Forward")
          (Utilities|FlowControl|Delay 2.0)
          (CallFunction|LookattheTv)
          (else
            (Variables|LookatDoor|SetbIsLookingDoor false)))))))

(event Custom|LookAtTheTv
  (Audio|SetSoundMixClassOverride "/Game/MELE/Blueprints/Audio/SCM_Meld.SCM_Meld" "/Game/MELE/Blueprints/Audio/SC_Voice_Meld.SC_Voice_Meld" 0.7 1.0 0.5 true)
  (bind (_direction _alpha) (Timeline|TimeLToDoor ReverseFromEnd)
    (:Update
      (Transformation|SetActorRotation (Math|Rotator|Lerp(Rotator) "0, 0, 0" (Variables|LookAtDoor|GetRotToDoor) _alpha true)))
    (:Finished
      (if (Utilities|Enum|Equal(Enum) _direction "Forward")
        (Utilities|FlowControl|Delay 2.0)
        (CallFunction|LookattheTv)
        (else
          (Variables|LookatDoor|SetbIsLookingDoor false))))))

(event EventBeginPlay
  (InitFunc|FRetrivePlayerPtr)
  (InitFunc|FRetriveGameModePtr))

(event EventTick
  (params (DeltaSeconds :type Float%20%28single-precision%29))
  (bind _gm_mainptr (Utilities|GetGMMain))
  (if (Default|FGetPartyinProgress _gm_mainptr)
    (CallFunction|FCalcJoie DeltaSeconds)
    (if (>= (Variables|Joie|GetJoieValue) 0.0)
      (CallFunction|FSetPostProcessDependonJoie)
      (else
        (Utilities|FlowControl|DoOnce false
          (:Completed
            (Default|TriggerLoseGame (Variables|Pointeur|GetGM_MainPtr))))))))

(event Input|KeyboardEvents|SpaceBar
  (params (Key :type Key%20Structure :default "None"))
  (:Pressed
    (bind _gm_mainptr (Utilities|GetGMMain))
    (if (and (Default|FGetPartyinProgress _gm_mainptr) (not (Variables|LookatDoor|GetbIsLookingDoor)))
      (CallFunction|FAddJoie)
      (Audio|PlaySound2D "/Game/MELE/Audios/S_FrappeStress.S_FrappeStress" 1.0 1.0 0.0 0 0))))

(event Input|MouseEvents|LeftMouseButton
  (params (Key :type Key%20Structure :default "None"))
  (:Pressed
    (bind _gm_mainptr (Utilities|GetGMMain))
    (if (Default|FGetPartyinProgress _gm_mainptr)
      (bind _playercontrollerptr (Utilities|GetPlayerController))
      (if (.ReturnValue (Game|Player|GetHitResultUnderCursorbyChannel _playercontrollerptr "TraceTypeQuery1" false))
        (bind _bsuccess (Class|BPIInteractible|FAction(Message) (.HitActor (Collision|BreakHitResult (.HitResult (Game|Player|GetHitResultUnderCursorbyChannel _playercontrollerptr "TraceTypeQuery1" false))))))
        (if _bsuccess
          (Math|Integer|DecrementInt (Variables|Joie|GetNbrBallon)))))))

(event Input|KeyboardEvents|P
  (params (Key :type Key%20Structure :default "None"))
  (:Pressed
    (bind _gm_mainptr (Utilities|GetGMMain))
    (if (Default|FGetPartyinProgress _gm_mainptr)
      (Default|FTogglePause _gm_mainptr))))

(event Input|KeyboardEvents|Escape
  (params (Key :type Key%20Structure :default "None"))
  (:Pressed
    (bind _gm_mainptr (Utilities|GetGMMain))
    (if (Default|FGetPartyinProgress _gm_mainptr)
      (Default|FTogglePause _gm_mainptr))))

(fn ConstructionScript
  (Variables|Joie|SetJoieValue (* (Variables|Joie|GetMaxJoieValue) (Variables|Joie|GetStartJoiePercent))))

(fn FCreateBallon
  (bind _currentballonptr (Variables|Pointeur|GetCurrentBallonPtr)
    (:then
      (bind _returnvalue (Default|InFlateBallon _currentballonptr 1.0))
      (if _returnvalue
        (Variables|Pointeur|SetCurrentBallonPtr 0)
        (Math|Integer|IncrementInt (Variables|Joie|GetNbrBallon)
          (:%20%20
            (return)))
        (else
          (return))))
    (:else
      (bind _returnvalue_2 (Game|SpawnActorfromClass "/Game/MELE/Blueprints/Ingrediant/BP_Ballon.BP_Ballon_C" (CallFunction|FBallonTransformSpawn) "Undefined" "MultiplyWithRoot" 0 0))
      (Variables|Pointeur|SetCurrentBallonPtr _returnvalue_2)
      (return))))

(fn FBallonTransformSpawn
  (bind _max_z (LocalVariables|GetMax%20Z))
  (bind _max_y (LocalVariables|GetMax%20Y))
  (bind _min_y (LocalVariables|GetMin%20Y))
  (bind _min_z (LocalVariables|GetMin%20Z))
  (bind _returnvalue (Math|Random|RandomFloatinRange _min_y _max_y))
  (bind _returnvalue_2 (Math|Random|RandomFloatinRange _min_z _max_z))
  (bind _returnvalue_3 (Math|Vector|MakeVector 2e+02 _returnvalue _returnvalue_2))
  (return (Math|Transform|MakeTransform _returnvalue_3 (Math|Rotator|FindLookatRotation _returnvalue_3 (Transformation|GetActorLocation)) "0.100000,0.100000,0.100000")))

(fn FGetJoiePercent
  (return (/ (Variables|Joie|GetJoieValue) (Variables|Joie|GetMaxJoieValue))))

(fn FRetrivePlayerPtr
  (bind _asplayer_controller (Utilities|Casting|CastToPlayerController (Pawn|GetController)))
  (Variables|Controller|SetPlayerControllerPtr _asplayer_controller))

(fn FRetriveGameModePtr
  (bind _asgm_main (Utilities|Casting|CastToGM_Main (Game|GetGameMode)))
  (bind _output_get (Variables|Pointeur|SetGM_MainPtr _asgm_main))
  (EventDispatchers|BindEventtoOnGameEnd _output_get (EventDispatchers|CreateEvent :!event FonEndGame)))

(fn FSetPostProcessDependonJoie
  (Utilities|Struct|SetmembersinPostProcessSettings (Variables|/Script/Engine.PostProcessComponent|GetSettings (Variables|Default|GetPostProcess)) (Math|Vector4|MakeVector4 1.0 1.0 1.0 (Math|Float|Clamp(Float) (Math|Float|Lerp 0.0 2.0 (Joie|FGetJoiePercent)) 0.0 2.0))))

(fn FCalcJoie
  (params (Deltatime :type Float%20%28double-precision%29))
  (bind _anxietyvalue (Variables|Joie|GetAnxietyValue))
  (bind _gm_mainptr (Variables|Pointeur|GetGM_MainPtr))
  ;[1 1 1] Retire la joie par rapport à l'anxiete
  (Variables|Joie|SetJoieValue (- (Variables|Joie|GetJoieValue) (* (Math|Float|SelectFloat (Math|Float|Lerp (/ _anxietyvalue 3.0) _anxietyvalue (Math|Float|Clamp(Float) (Default|FGetInfoDurationTime _gm_mainptr) 1.0 2.5)) 2.0 (Default|FGetIsInfo _gm_mainptr)) Deltatime)))
  (return))

(fn FAddJoie
  ;[1 1 1] Ajout la joie par rapport au ballon
  (Variables|Joie|SetJoieValue (+ (Variables|Joie|GetJoieValue) (* (Variables|Joie|GetBallonJoie) (Variables|Joie|GetNbrBallon))))
  (Math|Integer|IncrementInt (Variables|Joie|GetNbrBallon)
    (:%20%20
      (Utilities|Time|SetTimerbyEvent (EventDispatchers|CreateEvent :!event FResetStep) (Variables|Joie|GetResetTimeStep))
      (if (>= (Variables|Joie|GetJoieValue) (Variables|Joie|GetMaxJoieValue))
        (Variables|Joie|SetJoieValue (Variables|Joie|GetMaxJoieValue))
        (CallFunction|LookingattheDoor)
        (return)
        (else
          (return))))))

(fn FLookatDoor
  (bind _returnvalue (Utilities|Time|SetTimerbyEvent (EventDispatchers|CreateEvent :!event Custom|LookingAtTheDoor) 1e+01 false 2.0 5.0))
  (Variables|LookatDoor|SetLookAtDoorHandle _returnvalue)
  (return))

(fn FonEndGame
  (Utilities|Time|ClearandInvalidateTimerbyHandle (Variables|LookatDoor|GetLookAtDoorHandle)))

(fn FResetStep
  (Variables|Joie|SetNbrBallon 0))