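; Main game mode that spawns the TV on BeginPlay and manages pause, game end and loss.
; Both endings share FStartEndGame, which fires OnGameEnd, clears timers, fades the camera and turns off the TV.
; Winding down normally then shows animated credits, while losing first drops a physics rope and shows none.
; Game-duration timer, TV info swapping and in-game widget setup are disconnected, though getters still read their state.
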(event Custom|TriggerEndGame
  (CallFunction|FStartEndGame)
  (Utilities|FlowControl|Delay (Variables|Default|GetFadeDuration))
  (CallFunction|DisplayEndScreen))

(event Custom|TriggerSwapTV)

(event Custom|TriggerLoseGame
  (CallFunction|FSpawnRope)
  (Utilities|FlowControl|Delay 1.3)
  (CallFunction|FStartEndGame)
  (Utilities|FlowControl|Delay (Variables|Default|GetFadeDuration)))

(event Custom|DisplayEndScreen
  (bind _returnvalue (UserInterface|CreateWidget "/Game/MELE/Widget/Menu/WBP_Credit.WBP_Credit_C" (Game|GetPlayerController 0)))
  (UserInterface|Viewport|AddtoViewport _returnvalue 0)
  (Class|UserWidget|PlayAnimationForward _returnvalue (Variables|/Game/MELE/Widget/Menu/WBP_Credit.WBP_Credit_C|GetA_Credit _returnvalue) 0.7 false))

(event EventBeginPlay
  (bind _returnvalue (Game|GetPlayerController 0))
  (Input|SetInputModeGameOnly _returnvalue true)
  (Variables|/Script/Engine.PlayerController|SetbShowMouseCursor _returnvalue true)
  (bind _returnvalue_2 (Game|SpawnActorfromClass "/Game/MELE/Blueprints/Ingrediant/BP_TV.BP_TV_C" (Math|Transform|MakeTransform (Variables|TVPtr|GetTVSpawnLocation)) "Undefined" "MultiplyWithRoot" 0 0))
  (Variables|TVPtr|SetTVPtr _returnvalue_2))

(fn ConstructionScript)

(fn FTogglePause
  (if (Game|IsGamePaused)
    ;[1 0 0] UnPause
    (Game|SetGamePaused false)
    (bind _widgetpauseptr (Variables|Default|GetWidgetPausePtr)
      (:then
        (Widget|SetVisibility _widgetpauseptr "Hidden")
        (Input|SetInputModeGameandUI (Game|GetPlayerController 0) (Variables|Default|GetInGameWidgetPtr) "DoNotLock" false true))
      (:else))
    (else
      ;[0.0403 1 0] Pause
      (Game|SetGamePaused true)
      (bind _widgetpauseptr_2 (Variables|Default|GetWidgetPausePtr)
        (:then
          (Widget|SetVisibility _widgetpauseptr_2 "Visible"))
        (:else
          (bind _returnvalue (UserInterface|CreateWidget "/Game/MELE/Widget/InGame/WBP_Pause.WBP_Pause_C" (Game|GetPlayerController 0)))
          (bind _output_get (Variables|Default|SetWidgetPausePtr _returnvalue))
          (UserInterface|Viewport|AddtoViewport _output_get 0)))
      (Input|SetInputModeGameandUI (Game|GetPlayerController 0) (Variables|Default|GetWidgetPausePtr) "DoNotLock" false true))))

(fn FInitinGameWidget
  (bind _returnvalue (Game|GetPlayerController 0))
  (bind _returnvalue_2 (UserInterface|CreateWidget "/Game/MELE/Widget/InGame/WBP_InGame.WBP_InGame_C" _returnvalue))
  (Variables|Default|SetInGameWidgetPtr _returnvalue_2)
  (Variables|/Script/Engine.PlayerController|SetbShowMouseCursor _returnvalue true)
  (bind _ingamewidgetptr (Variables|Default|GetInGameWidgetPtr)
    (:then
      (UserInterface|Viewport|AddtoViewport _ingamewidgetptr 0)
      (Input|SetInputModeGameandUI 0 0 "DoNotLock" false false))
    (:else
      (Class|AutomationBlueprintFunctionLibrary|AddExpectedLogError "Wesh le Widget à pas réussi à se create"))))

(fn FGetPartyTimeRemaining
  (return (Utilities|Time|GetTimerRemainingTimebyHandle (Variables|Default|GetGameDurationHandle))))

(fn FGetIsInfo
  (return (Variables|Default|GetbIsInfo)))

(fn FGetInfoDurationTime
  (return (Class|KismetSystemLibrary|GetTimerElapsedTimeHandle (Variables|Default|GetGameDurationHandle))))

(fn FGetPartyinProgress
  (return (not (Variables|Default|GetbIsFinish))))

(fn FStartEndGame
  (Default|CallOnGameEnd)
  (Utilities|Time|ClearandInvalidateTimerbyHandle (Variables|Default|GetGameDurationHandle))
  (Utilities|Time|ClearandInvalidateTimerbyHandle (Variables|TVPtr|GetTriggerSwapTVHandle))
  (Variables|Default|SetbIsFinish true)
  (CameraFades|StartCameraFade :self (Game|GetPlayerCameraManager 0) :ToAlpha 1.0 :Duration (Variables|Default|GetFadeDuration) :bShouldFadeAudio true :bHoldWhenFinished true)
  (Default|TurnOffTv (Variables|TVPtr|GetTVPtr))
  (return))

(fn FSpawnRope
  (bind _returnvalue (Game|SpawnActorfromClass "/Game/MELE/Blueprints/Ingrediant/BP_Rope.BP_Rope_C" (Math|Transform|MakeTransform (LocalVariables|GetSpawnLocation) (LocalVariables|GetSpawnRotation)) "Undefined" "MultiplyWithRoot" 0 0))
  (Default|SimuPhys _returnvalue))