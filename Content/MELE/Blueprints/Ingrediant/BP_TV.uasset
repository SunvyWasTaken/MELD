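; BP_TV is a TV actor that plays a sequence of audio lines and quizzes the player between them.
; An integer "Line" parameter selects each clip on the audio component, starting at BeginPlay.
; When audio finishes, the first line auto-advances; later ones open a WBP_Question widget, where a correct answer advances and a wrong one replays.
; TurnOffTv switches the media player to an off-screen source, while video-swap logic sits unconnected.
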(event OnAudioFinished(S_TV_Cue)
  (if (>= (Variables|Default|GetCurrentLine) 1)
    (bind _returnvalue (UserInterface|CreateWidget "/Game/MELE/Widget/InGame/WBP_Question.WBP_Question_C" (Game|GetPlayerController 0)))
    (UserInterface|Viewport|AddtoViewport _returnvalue 0)
    (EventDispatchers|AssignOnAnswer _returnvalue (delegate Custom|OnAnswer_Event))
    (Default|Creatiobn _returnvalue)
    (else
      (Math|Integer|IncrementInt (Variables|Default|GetCurrentLine)
        (:%20%20
          (CallFunction|ToggleVideo))))))

(event Custom|ToggleVideo
  (Effects|Components|ParticleSystem|SetIntParameter (Variables|Default|GetS_TV_Cue) "Line" (Variables|Default|GetCurrentLine))
  (Audio|Components|Audio|Play (Variables|Default|GetS_TV_Cue) 0.0))

(event Custom|TurnOffTv
  (Media|MediaPlayer|OpenSource (Variables|Default|GetMediaPlayerRef) "/Game/Movies/TurnOffTVScreen.TurnOffTVScreen"))

(event Custom|OnAnswer_Event
  (params (Correct :type Boolean))
  (if Correct
    (Math|Integer|IncrementInt (Variables|Default|GetCurrentLine)
      (:%20%20
        _)))
  (CallFunction|ToggleVideo))

(event EventBeginPlay
  (CallFunction|FRetriveGameModePtr)
  (CallFunction|ToggleVideo))

(fn ConstructionScript)

(fn FRetriveGameModePtr
  (bind _asgm_main (Utilities|Casting|CastToGM_Main (Game|GetGameMode)))
  (Variables|Pointeur|SetGM_MainPtr _asgm_main))