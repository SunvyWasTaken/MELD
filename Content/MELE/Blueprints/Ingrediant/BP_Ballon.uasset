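; BP_Ballon is an inflatable balloon actor in the MELE ingredient set that grows in stages and can be destroyed by an action.
; InFlateBallon raises CurrentAlpha by a percentage step and reports whether it has reached full inflation.
; Each Tick eases the actor scale at constant speed toward a size lerped from zero to full by CurrentAlpha, so growth looks smooth.
; FAction destroys the balloon and returns true.
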(event EventTick
  (params (DeltaSeconds :type Float%20%28single-precision%29))
  (CallFunction|TickSetScaleDependonAlpha DeltaSeconds))

(fn ConstructionScript)

(fn TickSetScaleDependonAlpha
  (params (DeltaTime :type Float%20%28single-precision%29))
  (Transformation|SetActorScale3D (Math|Interpolation|VInterptoConstant (Transformation|GetActorScale3D) (Math|Vector|Lerp(Vector) "0, 0, 0" "1.000000,1.000000,1.000000" (Variables|Default|GetCurrentAlpha)) DeltaTime 1.0))
  (return))

(fn InFlateBallon
  (Variables|Default|SetCurrentAlpha (+ (Variables|Default|GetCurrentAlpha) (/ (Variables|Default|GetAddPercent) 1e+02)))
  (return (>= (Variables|Default|GetCurrentAlpha) 1.0)))

(fn FAction
  (Actor|DestroyActor)
  (return true))